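; Test Blueprint that visualizes movement math derived from two handles, left and right.
; Each tick, dot products of handle forward vectors with world X and Z yield differential terms that spin two tester components around yaw and roll axes.
; ForwardStrength scales with combined handle tilt, fading as the differential grows, and points from the actor toward the handle extremities' midpoint.
; A marker component follows that midpoint.
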(event EventTick
  (params (DeltaSeconds :type Float%20%28single-precision%29))
  (CallFunction|UpdateRotation DeltaSeconds)
  (CallFunction|UpdatePosition DeltaSeconds)
  (CallFunction|UpdateHandlesMidPointLocation))

(fn ConstructionScript)

(fn GetAngularAngleXY
  (params (Reference :type Scene%20Component%20Object%20Reference))
  (return (Math|Vector|DotProduct "1.000000, 0,0.000000" (Math|Vector|GetForwardVector Reference))))

(fn GetTotalAngularAngleXY
  (return (+ (CallFunction|GetAngularAngleXY (Variables|Default|GetHandleL)) (- 0.0 (CallFunction|GetAngularAngleXY (Variables|Default|GetHandleR))))))

(fn GetAngularAngleYZ
  (params (Reference :type Scene%20Component%20Object%20Reference))
  (return (Math|Vector|DotProduct "0.000000, 0,1.000000" (Math|Vector|GetForwardVector Reference))))

(fn GetTotalAngularAngleYZ
  (return (+ (- 0.0 (CallFunction|GetAngularAngleYZ (Variables|Default|GetHandleL))) (CallFunction|GetAngularAngleYZ (Variables|Default|GetHandleR)))))

(fn UpdateRotation
  (params (DeltaSeconds :type Float%20%28single-precision%29))
  (bind _rotationstrength (Variables|Default|GetRotationStrength))
  (Transformation|AddRelativeRotation (Variables|Default|GetAngularAngleTesterXY) (Math|Vector|RotatorfromAxisandAngle "0, 0,1.000000" (* DeltaSeconds (CallFunction|GetTotalAngularAngleXY) _rotationstrength)) false false)
  (Transformation|AddRelativeRotation (Variables|Default|GetAngularAngleTesterYZ) (Math|Vector|RotatorfromAxisandAngle "1.000000, 0, 0" (* DeltaSeconds (CallFunction|GetTotalAngularAngleYZ) _rotationstrength)) false false))

(fn UpdatePosition
  (params (DeltaSeconds :type Float%20%28single-precision%29))
  (bind _handler (Variables|Default|GetHandleR))
  (bind _handlel (Variables|Default|GetHandleL))
  (bind _forwardstrength (Variables|Default|GetForwardStrength))
  (Transformation|SetRelativeScale3D _forwardstrength (* "1.000000,1.000000,1.000000" (Math|Float|Lerp (* DeltaSeconds (Variables|Default|GetMoveStrength) (Math|Float|Absolute(Float) (/ (+ (+ (CallFunction|GetAngularAngleXY _handlel) (CallFunction|GetAngularAngleXY _handler)) (+ (CallFunction|GetAngularAngleYZ _handlel) (CallFunction|GetAngularAngleYZ _handler))) 2.0))) 0.0 (Math|Float|Clamp(Float) (/ (+ (CallFunction|GetTotalAngularAngleXY) (CallFunction|GetTotalAngularAngleYZ)) 2.0)))))
  (Transformation|SetWorldRotation _forwardstrength (Math|Rotator|MakeRotfromXZ (CallFunction|GetMoveWorldDirection) (Math|Vector|MakeVector 0.0 0.0 1.0)) false false))

(fn GetMoveWorldDirection
  (return (Math|Vector|Normalize (- (CallFunction|GetHandlesExtremityMidPointWorldLocation) (Transformation|GetActorLocation)))))

(fn GetHandlesExtremityMidPointWorldLocation
  (bind _handleextemityr (Variables|Default|GetHandleExtemityR))
  (bind _returnvalue (Transformation|GetWorldLocation _handleextemityr))
  (return (+ (/ (- (Transformation|GetWorldLocation (Variables|Default|GetHandleExtremityL)) _returnvalue) 2.0) _returnvalue)))

(fn UpdateHandlesMidPointLocation
  (Transformation|SetWorldLocation (Variables|Default|GetHandlesMidPoint) (CallFunction|GetHandlesExtremityMidPointWorldLocation) false false))